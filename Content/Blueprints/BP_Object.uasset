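; BP_Object is an inspectable actor that moves up to the first-person player when interacted with and returns afterward.
; Interact makes the player's capsule ignore WorldStatic, locks movement and flags inspection.
; The MoveObject timeline then lerps the actor from its BeginPlay transform to the player's Sphere location and camera rotation, calling TimelineFinished on the character when done.
; StopInspection reverses the same timeline.
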(event `self.ReceiveBeginPlay`
  (set `self.InitialTransform` (`SceneComponent.K2_GetComponentToWorld` (`self.DefaultSceneRoot`)))
  (bind _asbp_first_person_character (cast `/Game/Blueprints/BP_FirstPersonCharacter` (`GameplayStatics.GetPlayerCharacter` 0)))
  (set `self.FirstPersonRef` _asbp_first_person_character))

(event `/Game/Blueprints/BPI_Interact.Interact`
  (bind _firstpersonref (`self.FirstPersonRef`))
  (bind (_initialtransform_location _initialtransform_rotation) (`KismetMathLibrary.BreakTransform` (`self.InitialTransform`)))
  (`PrimitiveComponent.SetCollisionResponseToChannel` (`Character.CapsuleComponent` _firstpersonref) "ECC_WorldStatic" "ECR_Ignore")
  (set `/Game/Blueprints/BP_FirstPersonCharacter.bCanMove` false _firstpersonref)
  (set `/Game/Blueprints/BP_FirstPersonCharacter.bIsInspecting` true _firstpersonref)
  (bind (_direction _forward) (`Timeline|MoveObject` :!label _label)
    (:`Update`
      (`self.K2_SetActorLocationAndRotation` self (`KismetMathLibrary.VLerp` _initialtransform_location (`SceneComponent.K2_GetComponentLocation` (`/Game/Blueprints/BP_FirstPersonCharacter.Sphere` _firstpersonref)) _forward) (`KismetMathLibrary.RLerp` _initialtransform_rotation (`SceneComponent.K2_GetComponentRotation` (`/Game/Blueprints/BP_FirstPersonCharacter.FirstPersonCamera` _firstpersonref)) _forward) false false))
    (:`Finished`
      (`/Game/Blueprints/BP_FirstPersonCharacter.TimelineFinished` _firstpersonref))))

(event `/Game/Blueprints/BPI_Interact.StopInspection`
  (goto _label :!via `Reverse`))

(fn `UserConstructionScript`)